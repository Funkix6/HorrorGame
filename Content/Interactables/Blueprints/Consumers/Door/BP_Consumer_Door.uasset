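; Lockable door interactable that swings open and shut, built on a parent consumer class.
; While locked, Interact defers to the parent's check, then either unlocks with a sound or plays a locked sound.
; Once unlocked, it plays or reverses a timeline that lerps rotation between the BeginPlay closed rotation and Open, toggling IsOpen on finish.
; Point sets the HUD cue to a closed or open lock icon.
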(event `self.ReceiveBeginPlay`
  (`parent.ReceiveBeginPlay`)
  (set `self.Closed` (`SceneComponent.K2_GetComponentRotation` (`self.Scene`))))

(fn `CloseDoor`
  (`GameplayStatics.PlaySoundAtLocation` "/Game/Interactables/Blueprints/Consumers/Door/S_DoorShut.S_DoorShut" (`self.K2_GetActorLocation`) (struct) 1.0 1.0 0.0 null null null null)
  (`TimelineComponent.Reverse` (`self.Timeline`)))

(fn `Interact`
  (params (Instigator :type "/Game/ThirdPerson/Blueprints/BP_ThirdPersonCharacter Object Reference"))
  (returns (Success :type Boolean))
  (if (`self.IsUnlocked?`)
    (if (`self.IsOpen?`)
      (`self.CloseDoor`)
      (else
        (`self.OpenDoor`)))
    (else
      (bind _success (`parent.Interact` Instigator))
      (if _success
        (`GameplayStatics.PlaySoundAtLocation` "/Game/Interactables/Blueprints/Consumers/Door/S_DoorUnlock.S_DoorUnlock" (`self.K2_GetActorLocation`) (struct) 1.0 1.0 0.0 null null null null)
        (set `self.IsUnlocked?` true)
        (else
          (`GameplayStatics.PlaySoundAtLocation` "/Game/Interactables/Blueprints/Consumers/Door/S_DoorLocked_Cue.S_DoorLocked_Cue" (`self.K2_GetActorLocation`) (struct) 1.0 1.0 0.0 null null null null)))
      (return false))))

(fn `OpenDoor`
  (`GameplayStatics.PlaySoundAtLocation` "/Game/Interactables/Blueprints/Consumers/Door/S_OpenDoor.S_OpenDoor" (`self.K2_GetActorLocation`) (struct) 1.0 1.0 0.0 null null null null)
  (`TimelineComponent.Play` (`self.Timeline`)))

(fn `Point`
  (params (Instigator :type "/Game/ThirdPerson/Blueprints/BP_ThirdPersonCharacter Object Reference"))
  (returns (Interactable :type "/Game/Interactables/Blueprints/BP_Interactable Object Reference"))
  (bind _interactable (`parent.Point` Instigator))
  (if (not (`self.IsUnlocked?`))
    (`/Game/ThirdPerson/UMG/WBP_HUD.SetInteractionCueIcon` (`/Game/ThirdPerson/Blueprints/BP_ThirdPersonCharacter.HUD` (`local.Instigator`)) "/Game/ThirdPerson/UMG/Icons/T_LockClose.T_LockClose")
    (else
      (`/Game/ThirdPerson/UMG/WBP_HUD.SetInteractionCueIcon` (`/Game/ThirdPerson/Blueprints/BP_ThirdPersonCharacter.HUD` (`local.Instigator`)) "/Game/ThirdPerson/UMG/Icons/T_LockOpen.T_LockOpen")))
  (return _interactable))

(fn `UserConstructionScript`
  (`parent.UserConstructionScript`))