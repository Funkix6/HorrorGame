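; BP_Consumer is an interactable actor that takes one unit of a configured item from whoever interacts with it.
; Interact looks up the ConsumedItem data table row, then asks the instigator's BPCStorage component to remove that item by name.
; The instigator's HUD shows the removed item's display name or a failure message through ShowRemovedItem, and Interact returns whether removal succeeded.
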(fn `Interact`
  (params (Instigator :type "/Game/ThirdPerson/Blueprints/BP_ThirdPersonCharacter Object Reference"))
  (returns (Success :type Boolean))
  (locals (Item :type "/Game/Interactables/Blueprints/DataStructures/S_Item Structure"))
  (bind (_datatable _rowname) (break `DataTableRowHandle` (`self.ConsumedItem`)))
  (bind _returnvalue (`|GetDataTableRow` _datatable _rowname)
    (:`then`
      (bind _output_get (set `local.Item` _returnvalue))
      (bind _success (`/Game/ThirdPerson/Blueprints/Inventory/BPC_Storage.RemoveItem` (`/Game/ThirdPerson/Blueprints/BP_ThirdPersonCharacter.BPC_Storage` (`local.Instigator`)) (`.Name_8_DF8AA319426642A456391FBB829ED52C` (break `/Game/Interactables/Blueprints/DataStructures/S_Item` _output_get)) 1))
      (if _success
        (`/Game/ThirdPerson/UMG/WBP_HUD.ShowRemovedItem` (`/Game/ThirdPerson/Blueprints/BP_ThirdPersonCharacter.HUD` (`local.Instigator`)) (`.DisplayName_3_60D975314E1A1365347F57994A4AB155` (break `/Game/Interactables/Blueprints/DataStructures/S_Item` (`local.Item`))))
        (return true)
        (else
          (`/Game/ThirdPerson/UMG/WBP_HUD.ShowRemovedItem` (`/Game/ThirdPerson/Blueprints/BP_ThirdPersonCharacter.HUD` (`local.Instigator`)) "This doesn't seem to be working...")
          (return false))))))

(fn `UserConstructionScript`
  (`parent.UserConstructionScript`))