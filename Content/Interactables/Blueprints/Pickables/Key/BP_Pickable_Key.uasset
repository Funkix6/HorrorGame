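; BP_Pickable_Key is a key pickup Blueprint that builds on a parent interactable class.
; Its Interact override runs the parent interaction, plays the S_Keys sound in 2D and returns the parent's result.
; The sound plays regardless of that result, and the event graph holds only disabled default events.
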(fn `Interact`
  (params (Instigator :type "/Game/ThirdPerson/Blueprints/BP_ThirdPersonCharacter Object Reference"))
  (returns (Success :type Boolean))
  (bind _success (`parent.Interact` Instigator))
  (`GameplayStatics.PlaySound2D` "/Game/Interactables/Blueprints/Pickables/Key/S_Keys.S_Keys" 1.0 1.0 0.0 null null)
  (return _success))

(fn `UserConstructionScript`
  (`parent.UserConstructionScript`))