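; BP_Pickable is an interactable item that the player picks up into their storage.
; Pointing at it runs the parent logic and sets the HUD interaction cue to a grab icon.
; Interacting looks up the item's data table row, adds the amount to the instigator's BPCStorage, shows the addition on the HUD, clears the pointed interactable and destroys the actor.
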(fn `Interact`
  (params (Instigator :type "/Game/ThirdPerson/Blueprints/BP_ThirdPersonCharacter Object Reference"))
  (returns (Success :type Boolean))
  (locals (HUD :type "/Game/ThirdPerson/UMG/WBP_HUD Object Reference") (Item :type "/Game/Interactables/Blueprints/DataStructures/S_Item Structure"))
  (bind (_datatable _rowname) (break `DataTableRowHandle` (`self.ItemData`)))
  (bind _returnvalue (`|GetDataTableRow` _datatable _rowname)
    (:`then`
      (bind _output_get (set `local.Item` _returnvalue))
      (bind _value (`/Game/ThirdPerson/Blueprints/Inventory/BPC_Storage.AddItem` (`/Game/ThirdPerson/Blueprints/BP_ThirdPersonCharacter.BPC_Storage` (`local.Instigator`)) (`.Name_8_DF8AA319426642A456391FBB829ED52C` (break `/Game/Interactables/Blueprints/DataStructures/S_Item` _output_get)) (`self.Amount`)))
      (`/Game/ThirdPerson/UMG/WBP_HUD.ShowAddedItem` (`/Game/ThirdPerson/Blueprints/BP_ThirdPersonCharacter.HUD` (`local.Instigator`)) (`self.Amount`) (`.DisplayName_3_60D975314E1A1365347F57994A4AB155` (break `/Game/Interactables/Blueprints/DataStructures/S_Item` (`local.Item`))) _value)
      (set `/Game/ThirdPerson/Blueprints/BP_ThirdPersonCharacter.PointedInteractable` null (`local.Instigator`))
      (`self.K2_DestroyActor`)
      (return true))))

(fn `Point`
  (params (Instigator :type "/Game/ThirdPerson/Blueprints/BP_ThirdPersonCharacter Object Reference"))
  (returns (Interactable :type "/Game/Interactables/Blueprints/BP_Interactable Object Reference"))
  (bind _interactable (`parent.Point` Instigator))
  (`/Game/ThirdPerson/UMG/WBP_HUD.SetInteractionCueIcon` (`/Game/ThirdPerson/Blueprints/BP_ThirdPersonCharacter.HUD` (`local.Instigator`)) "/Game/ThirdPerson/UMG/Icons/T_GrabIcon.T_GrabIcon")
  (return _interactable))

(fn `UserConstructionScript`
  (`parent.UserConstructionScript`))