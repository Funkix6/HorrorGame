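; BP_Readable_Letter is a readable letter interactable that adds paper sounds to the interaction inherited from its parent Blueprint.
; Interact runs the parent logic, then plays a 2D unfold sound if IsGrabbed is true or a fold sound otherwise, and returns true.
; The event graph holds only disabled default events, and the construction script just calls the parent.
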(fn `Interact`
  (params (Instigator :type "/Game/ThirdPerson/Blueprints/BP_ThirdPersonCharacter Object Reference"))
  (returns (Success :type Boolean))
  (`parent.Interact` Instigator)
  (if (`self.IsGrabbed?`)
    (`GameplayStatics.PlaySound2D` "/Game/Interactables/Blueprints/Readables/Sound/S_PaperUnfold.S_PaperUnfold" 1.0 1.0 0.0 null null)
    (else
      (`GameplayStatics.PlaySound2D` "/Game/Interactables/Blueprints/Readables/Sound/S_PaperFold.S_PaperFold" 1.0 1.0 0.0 null null)))
  (return true))

(fn `UserConstructionScript`
  (`parent.UserConstructionScript`))