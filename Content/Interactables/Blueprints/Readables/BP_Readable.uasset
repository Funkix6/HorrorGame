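; BP_Readable is an interactable object the player can pick up to read in front of the camera and put back.
; Interact toggles it: grabbing places it just ahead of the instigator's follow camera, facing it, attaches it there and disables movement.
; Interacting again detaches it, restores the transform saved on BeginPlay and re-enables walking.
; Point shows an eye cue icon, or hides the cue while held.
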(event `self.ReceiveBeginPlay`
  (set `self.InitialTransform` (`self.GetTransform`)))

(fn `Interact`
  (params (Instigator :type "/Game/ThirdPerson/Blueprints/BP_ThirdPersonCharacter Object Reference"))
  (returns (Success :type Boolean))
  (if (not (`self.IsGrabbed?`))
    (`self.PlaceReadable` Instigator)
    (set `self.IsGrabbed?` true)
    (`CharacterMovementComponent.DisableMovement` (`Character.CharacterMovement` (`local.Instigator`)))
    (else
      (`self.K2_DetachFromActor` "KeepWorld" "KeepWorld" "KeepWorld")
      (`self.K2_SetActorTransform` (`self.InitialTransform`))
      (set `self.IsGrabbed?` false)
      (`CharacterMovementComponent.SetMovementMode` (`Character.CharacterMovement` (`local.Instigator`)) "MOVE_Walking" 0)))
  (return true))

(fn `PlaceReadable`
  (params (Instigator :type "/Game/ThirdPerson/Blueprints/BP_ThirdPersonCharacter Object Reference"))
  (bind _followcamera (`/Game/ThirdPerson/Blueprints/BP_ThirdPersonCharacter.FollowCamera` Instigator))
  (bind _returnvalue (+ (`SceneComponent.K2_GetComponentLocation` _followcamera) (* 35.0 (`SceneComponent.GetForwardVector` _followcamera))))
  (`self.K2_SetActorLocation` _returnvalue)
  (`self.K2_SetActorRotation` (`KismetMathLibrary.FindLookAtRotation` _returnvalue (`SceneComponent.K2_GetComponentLocation` (`/Game/ThirdPerson/Blueprints/BP_ThirdPersonCharacter.FollowCamera` (`local.Instigator`)))))
  (`self.K2_AttachToComponent` (`/Game/ThirdPerson/Blueprints/BP_ThirdPersonCharacter.FollowCamera` (`local.Instigator`)) "None" "KeepWorld" "KeepWorld" "KeepWorld"))

(fn `Point`
  (params (Instigator :type "/Game/ThirdPerson/Blueprints/BP_ThirdPersonCharacter Object Reference"))
  (returns (Interactable :type "/Game/Interactables/Blueprints/BP_Interactable Object Reference"))
  (bind _interactable (`parent.Point` Instigator))
  (if (`self.IsGrabbed?`)
    (`/Game/ThirdPerson/UMG/WBP_HUD.DisplayInteractionCue` (`/Game/ThirdPerson/Blueprints/BP_ThirdPersonCharacter.HUD` (`local.Instigator`)) false)
    (else
      (`/Game/ThirdPerson/UMG/WBP_HUD.SetInteractionCueIcon` (`/Game/ThirdPerson/Blueprints/BP_ThirdPersonCharacter.HUD` (`local.Instigator`)) "/Game/Interactables/Blueprints/Readables/Textures/Icons/T__Eye.T__Eye")))
  (return _interactable))

(fn `UserConstructionScript`
  (`parent.UserConstructionScript`))